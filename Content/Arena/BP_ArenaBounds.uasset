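; BP_ArenaBounds is an arena boundary actor that keeps two fighters inside a circular area.
; InitializeArenaFromFighters stores both fighter references and moves the actor to their horizontal midpoint, keeping its own height.
; Every Tick, ClampActorToArena limits each valid fighter's XY offset from the center to ArenaRadius, preserving Z and repositioning without sweep.
; Tick also draws a debug sphere showing the radius.
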(event `self.ReceiveTick`
  (params (DeltaSeconds :type "Float (single-precision)"))
  (`self.ClampActorToArena` (`self.P1Ref`))
  (`self.ClampActorToArena` (`self.P2Ref`))
  (`KismetSystemLibrary.DrawDebugSphere` (`self.K2_GetActorLocation`) (`self.ArenaRadius`) 64 (struct :`R` 1.0 :`G` 1.0 :`B` 1.0 :`A` 1.0) 0.0 5.0))

(fn `ClampActorToArena`
  (params (TargetActor :type "Actor Object Reference"))
  (bind _returnvalue (`self.K2_GetActorLocation` TargetActor))
  (bind _returnvalue_2 (`self.K2_GetActorLocation`))
  (`/Game/EditorBlueprintResources/StandardMacros.IsValid` TargetActor
    (:`Is Valid`
      (`self.K2_SetActorLocation` TargetActor (`KismetMathLibrary.MakeVector` (.x (+ (`KismetMathLibrary.ClampVectorSize` (`KismetMathLibrary.MakeVector` (.x (- _returnvalue _returnvalue_2)) (.y (- _returnvalue _returnvalue_2))) 0.0 (`self.ArenaRadius`)) _returnvalue_2)) (.y (+ (`KismetMathLibrary.ClampVectorSize` (`KismetMathLibrary.MakeVector` (.x (- _returnvalue _returnvalue_2)) (.y (- _returnvalue _returnvalue_2))) 0.0 (`self.ArenaRadius`)) _returnvalue_2)) (.z _returnvalue)) false false))))

(fn `InitializeArenaFromFighters`
  (params (P1 :type "Actor Object Reference") (P2 :type "Actor Object Reference"))
  (bind _output_get (set `self.P1Ref` P1))
  (bind _output_get_2 (set `self.P2Ref` P2))
  (`self.K2_SetActorLocation` (`KismetMathLibrary.MakeVector` (.x (* (+ (`self.K2_GetActorLocation` _output_get_2) (`self.K2_GetActorLocation` _output_get)) 0.5)) (.y (* (+ (`self.K2_GetActorLocation` _output_get_2) (`self.K2_GetActorLocation` _output_get)) 0.5)) (.z (`self.K2_GetActorLocation`))) true))

(fn `UserConstructionScript`)